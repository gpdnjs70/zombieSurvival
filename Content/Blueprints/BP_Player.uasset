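; BP_Player is the player character Blueprint, handling basic movement through Enhanced Input.
; BeginPlay adds the IMC_PlayerInput mapping context, and the IA_Vertical and IA_Horizontal actions feed Add Movement Input.
; Their direction vectors take only control-rotation roll and pitch respectively, with yaw zeroed, so movement follows world X and Y regardless of where the controller faces.
; Two MaxWalkSpeed setters are unconnected and never run.
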(event Input|EnhancedActionEvents|EnhancedInputActionIA_Vertical
  (params (ActionValue :type Float%20%28double-precision%29) (ElapsedSeconds :type Float%20%28double-precision%29) (TriggeredSeconds :type Float%20%28double-precision%29) (InputAction :type Input%20Action%20Object%20Reference :default "/Game/Inputs/Actions/IA_Vertical.IA_Vertical"))
  (Pawn|Input|AddMovementInput (Math|Vector|GetForwardVector (Math|Rotator|MakeRotator (.roll (Pawn|GetControlRotation :!class /Script/Engine.Pawn)) 0.0 0.0)) ActionValue false))

(event Input|EnhancedActionEvents|EnhancedInputActionIA_Horizontal
  (params (ActionValue :type Float%20%28double-precision%29) (ElapsedSeconds :type Float%20%28double-precision%29) (TriggeredSeconds :type Float%20%28double-precision%29) (InputAction :type Input%20Action%20Object%20Reference :default "/Game/Inputs/Actions/IA_Horizontal.IA_Horizontal"))
  (Pawn|Input|AddMovementInput (Math|Vector|GetRightVector (Math|Rotator|MakeRotator 0.0 (.pitch (Pawn|GetControlRotation :!class /Script/Engine.Pawn)) 0.0)) ActionValue false))

(event EventBeginPlay
  ;[0.06047 0.0531 0.15 0.5] Input Mapping Context 초기 설정
  (Input|AddMappingContext (PlayerController|LocalPlayerSubsystems|GetEnhancedInputLocalPlayerSubsystem (Game|GetPlayerController 0)) "/Game/Inputs/IMC_PlayerInput.IMC_PlayerInput" 0 "(bIgnoreAllPressedKeysUntilRelease=True,bForceImmediately=False,bNotifyUserSettings=False)"))

(event Collision|EventActorBeginOverlap
  (params (OtherActor :type Actor%20Object%20Reference)))

(event EventTick
  (params (DeltaSeconds :type Float%20%28single-precision%29)))

(fn ConstructionScript)